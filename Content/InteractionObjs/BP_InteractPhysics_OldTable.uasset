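; Interactable physics prop of an old table with four box parts, configured entirely in the Construction Script.
; One TableMaterial setting is applied to the table and to both material slots of each box.
; Each box has its own check that, when false, disables its collision and physics and hides it, allowing table variants per instance.
; The event graph holds no active logic.
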(event EventBeginPlay)

(event Collision|EventActorBeginOverlap
  (params (OtherActor :type Actor%20Object%20Reference)))

(event EventTick
  (params (DeltaSeconds :type Float%20%28single-precision%29)))

(fn ConstructionScript
  (bind _tablebox1 (Variables|Default|GetTableBox1))
  (bind _tablebox2 (Variables|Default|GetTableBox2))
  (bind _tablebox3 (Variables|Default|GetTableBox3))
  (bind _tablebox4 (Variables|Default|GetTableBox4))
  (bind _tablebox1_2 (Variables|Default|GetTableBox1))
  (bind _tablebox2_2 (Variables|Default|GetTableBox2))
  (bind _tablebox3_2 (Variables|Default|GetTableBox3))
  (bind _tablebox4_2 (Variables|Default|GetTableBox4))
  (bind _tablematerial (Variables|DesignFeatures|GetTableMaterial))
  (bind _materialinterface (Utilities|Struct|BreakStaticMaterial _tablematerial))
  (Rendering|Material|SetMaterial (Variables|Default|GetTable) 0 _materialinterface)
  (Rendering|Material|SetMaterial _tablebox1_2 0 _materialinterface)
  (Rendering|Material|SetMaterial _tablebox1_2 1 _materialinterface)
  (Rendering|Material|SetMaterial _tablebox2_2 0 _materialinterface)
  (Rendering|Material|SetMaterial _tablebox2_2 1 _materialinterface)
  (Rendering|Material|SetMaterial _tablebox3_2 0 _materialinterface)
  (Rendering|Material|SetMaterial _tablebox3_2 1 _materialinterface)
  (Rendering|Material|SetMaterial _tablebox4_2 0 _materialinterface)
  (Rendering|Material|SetMaterial _tablebox4_2 1 _materialinterface)
  (Utilities|FlowControl|Sequence
    (:then_0
      (if (not (Variables|DesignFeatures|GetTableBox_1))
        (Collision|SetCollisionEnabled _tablebox1 "NoCollision")
        (Rendering|SetVisibility _tablebox1 false false)
        (Development|SetHiddeninGame _tablebox1 true false)
        (Physics|SetSimulatePhysics _tablebox1 false)))
    (:then_1
      (if (not (Variables|DesignFeatures|GetTableBox_2))
        (Collision|SetCollisionEnabled _tablebox2 "NoCollision")
        (Rendering|SetVisibility _tablebox2 false false)
        (Development|SetHiddeninGame _tablebox2 true false)
        (Physics|SetSimulatePhysics _tablebox2 false)))
    (:then_2
      (if (not (Variables|DesignFeatures|GetTableBox_3))
        (Collision|SetCollisionEnabled _tablebox3 "NoCollision")
        (Rendering|SetVisibility _tablebox3 false false)
        (Development|SetHiddeninGame _tablebox3 true false)
        (Physics|SetSimulatePhysics _tablebox3 false)))
    (:then_3
      (if (not (Variables|DesignFeatures|GetTableBox_4))
        (Collision|SetCollisionEnabled _tablebox4 "NoCollision")
        (Rendering|SetVisibility _tablebox4 false false)
        (Development|SetHiddeninGame _tablebox4 true false)
        (Physics|SetSimulatePhysics _tablebox4 false)))))