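; BP_InteractPhysics_Door is a configurable physics-constrained door, set up entirely in its construction script.
; It applies the chosen door mesh and material, plus an optional decal mesh.
; ForwardOrBackward flips MoveToOpen's rotation and selects which constraint pair gets a limited swing: the door-frame pair or the other pair.
; The opposite pair's swing is set free, though each branch updates only one side of MoveToOpen's orientation.
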(event EventBeginPlay)

(event Collision|EventActorBeginOverlap
  (params (OtherActor :type Actor%20Object%20Reference)))

(event EventTick
  (params (DeltaSeconds :type Float%20%28single-precision%29)))

(fn ConstructionScript
  (bind _door (Variables|Default|GetDoor))
  (bind _movetoopen (Variables|Default|GetMoveToOpen))
  (bind _physicsconstraint (Variables|Default|GetPhysicsConstraint))
  (bind _decal (Variables|Default|GetDecal))
  (Components|StaticMesh|SetStaticMesh _door (Variables|DesignFeatures|GetDoorMesh))
  (Rendering|Material|SetMaterial _door 0 (Variables|DesignFeatures|GetDoorMaterial))
  (if (Variables|DesignFeatures|GetForwardOrBackward)
    (Transformation|SetRelativeRotation _movetoopen "0,90.000000, 0" false false)
    (Class|PhysicsConstraintComponent|SetAngularSwing1Limit (Variables|Default|GetDoorFrameConstraint1) "ACM_Limited" 45.0)
    (Class|PhysicsConstraintComponent|SetAngularSwing1Limit _physicsconstraint "ACM_Free" 0.0)
    (else
      (Transformation|SetRelativeRotation _movetoopen "0,-90.000000, 0" false false)
      (Class|PhysicsConstraintComponent|SetAngularSwing1Limit _physicsconstraint "ACM_Limited" 45.0)
      (Class|PhysicsConstraintComponent|SetAngularSwing1Limit (Variables|Default|GetDoorFrameConstraint2) "ACM_Free" 0.0)))
  (if (Variables|DesignFeatures|GetSetDecal?)
    (Components|StaticMesh|SetStaticMesh _decal (Variables|DesignFeatures|GetDecalForDoor))
    (else
      (Components|StaticMesh|SetStaticMesh _decal 0))))