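; PUPISettings is a component that configures the PUPI pick-up and inspect actor hosted in a named child actor component on its owner.
; On BeginPlay it finds that child, passes it the motion controller hand and main, pick-up and inspect settings, then initializes its variables.
; To cover BeginPlay ordering, it first overwrites the first input consumer with one spawned for the correct hand (none, left or right) if the hands differ.
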(event EventBeginPlay
  ;[1 1 1] Go through every child of Actor, PUPISettingsComponent is added to.
  (bind _array_element (Utilities|Array|ForEachLoopwithBreak (Components|GetChildrenComponents (VehicleSound|GetRootComponent (Components|GetOwner)) true) :!label _label)
    (:LoopBody
      (if (Utilities|Name|Equal(Name) (Utilities|String|StringToName (Utilities|GetObjectName _array_element)) (Variables|Default|GetPUPI_ChildActorName)) ; Find child with the name [PUPIChildActorName]
        (bind _aschild_actor_component (Utilities|Casting|CastToChildActorComponent _array_element))
        (bind _aspupi (Utilities|Casting|CastToPUPI (Variables|/Script/Engine.ChildActorComponent|GetChildActor _aschild_actor_component)))
        (Variables|Default|SetTargetPUPI _aspupi)
        (|ReplaceInputConsumers[0]
          (:%20%20
            (Variables|/Game/PickUpPlusInspect/Blueprint/PUPI.PUPI_C|SetMotionControllerHand (Variables|Default|GetTargetPUPI) (Variables|Default|GetMotionControllerHand))
            (Variables|/Game/PickUpPlusInspect/Blueprint/PUPI.PUPI_C|SetPUPISettings (Variables|Default|GetTargetPUPI) (Utilities|Struct|MakePUPISettings (Variables|Default|GetMainSettings) (Variables|Default|GetPickUpSettings) (Variables|Default|GetInspectSettings)))
            (Default|InitializeVariables (Variables|Default|GetTargetPUPI))
            (goto _label Break)))))))